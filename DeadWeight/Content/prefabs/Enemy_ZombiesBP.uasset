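; Zombie enemy that chases the player while in AJ mode and either kills them or is killed on contact.
; The Approach volume toggles chasing, and Tick reissues AI MoveTo toward the player while it is set.
; The game mode's RadioOn flag halts movement.
; Overlapping the Death volume restarts the level if IsAJChar is set, otherwise the zombie is destroyed (Brian's kill).
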(event OnComponentBeginOverlap(Death)
  (params (OverlappedComponent :type Primitive%20Component%20Object%20Reference) (OtherActor :type Actor%20Object%20Reference) (OtherComp :type Primitive%20Component%20Object%20Reference) (OtherBodyIndex :type Integer) (bFromSweep :type Boolean) (SweepResult :type Hit%20Result%20Structure%20%28by%20ref%29))
  ;[1 1 1] AJ Dies/Brian Kills Overlap
  (Utilities|Casting|CastToAJprefab_Blueprint OtherActor)
  (bind _asdwgame_mode (Utilities|Casting|CastToDWGameMode (Game|GetGameMode)))
  (if (Variables|/Game/UI/DWGameMode.DWGameMode_C|GetIsAJChar _asdwgame_mode)
    (bind _returnvalue (Game|GetCurrentLevelName true))
    (Game|OpenLevel(byName) (Utilities|String|StringToName _returnvalue))
    (else
      (Actor|DestroyActor))))

(event OnComponentBeginOverlap(Approach)
  (params (OverlappedComponent :type Primitive%20Component%20Object%20Reference) (OtherActor :type Actor%20Object%20Reference) (OtherComp :type Primitive%20Component%20Object%20Reference) (OtherBodyIndex :type Integer) (bFromSweep :type Boolean) (SweepResult :type Hit%20Result%20Structure%20%28by%20ref%29))
  ;[1 1 1] Zombie Chase AI
  (Utilities|Casting|CastToAJprefab_Blueprint OtherActor)
  (bind _asdwgame_mode (Utilities|Casting|CastToDWGameMode (Game|GetGameMode)))
  (if (Variables|/Game/UI/DWGameMode.DWGameMode_C|GetIsAJChar _asdwgame_mode)
    (Variables|Default|SetIsChasing true)))

(event OnComponentEndOverlap(Approach)
  (params (OverlappedComponent :type Primitive%20Component%20Object%20Reference) (OtherActor :type Actor%20Object%20Reference) (OtherComp :type Primitive%20Component%20Object%20Reference) (OtherBodyIndex :type Integer))
  ;[1 1 1] Zombie Chase AI
  (Utilities|Casting|CastToAJprefab_Blueprint OtherActor)
  (bind _asdwgame_mode (Utilities|Casting|CastToDWGameMode (Game|GetGameMode)))
  (if (Variables|/Game/UI/DWGameMode.DWGameMode_C|GetIsAJChar _asdwgame_mode)
    (Variables|Default|SetIsChasing false)))

(event Custom|MoveToPlayer
  ;[1 1 1] Zombie Chase AI
  (bind _asdwgame_mode (Utilities|Casting|CastToDWGameMode (Game|GetGameMode)))
  (if (not (Variables|/Game/UI/DWGameMode.DWGameMode_C|GetRadioOn _asdwgame_mode))
    (AI|AIMoveTo self "0, 0, 0" (Game|GetPlayerCharacter 0) 1.0 false)))

(event EventTick
  (params (DeltaSeconds :type Float%20%28single-precision%29))
  ;[1 1 1] Zombie Chase AI
  (bind _asdwgame_mode (Utilities|Casting|CastToDWGameMode (Game|GetGameMode)))
  (if (Variables|/Game/UI/DWGameMode.DWGameMode_C|GetRadioOn _asdwgame_mode)
    (Components|Movement|StopMovementImmediately (Variables|Character|GetCharacterMovement))
    (elif (Variables|Default|GetIsChasing)
      (CallFunction|MovetoPlayer))))

(fn ConstructionScript)