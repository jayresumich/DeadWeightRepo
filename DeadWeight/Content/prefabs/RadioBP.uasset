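; Radio prop Blueprint that marks when the AJ character is close enough to interact and shows a click prompt.
; Overlap events on RadColl set the AJInteract flag in DWGameMode and add or remove a ClickPrompt widget, only while IsAJChar is true.
; Tick removes the prompt whenever AJ is not the current character, without clearing AJInteract.
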(event OnComponentBeginOverlap(RadColl)
  (params (OverlappedComponent :type Primitive%20Component%20Object%20Reference) (OtherActor :type Actor%20Object%20Reference) (OtherComp :type Primitive%20Component%20Object%20Reference) (OtherBodyIndex :type Integer) (bFromSweep :type Boolean) (SweepResult :type Hit%20Result%20Structure%20%28by%20ref%29))
  ;[1 1 1] Can AJ Interact?
  (Utilities|Casting|CastToAJprefab_Blueprint OtherActor)
  (bind _asdwgame_mode (Utilities|Casting|CastToDWGameMode (Game|GetGameMode)))
  (if (Variables|/Game/UI/DWGameMode.DWGameMode_C|GetIsAJChar _asdwgame_mode)
    (bind _asdwgame_mode_2 (Utilities|Casting|CastToDWGameMode (Game|GetGameMode)))
    (Variables|/Game/UI/DWGameMode.DWGameMode_C|SetAJInteract _asdwgame_mode_2 true)
    (bind _returnvalue (UserInterface|CreateWidget "/Game/UI/ClickPrompt.ClickPrompt_C"))
    (bind _output_get (Variables|Default|SetClickPrompt _returnvalue))
    (UserInterface|Viewport|AddtoViewport _returnvalue 0)))

(event OnComponentEndOverlap(RadColl)
  (params (OverlappedComponent :type Primitive%20Component%20Object%20Reference) (OtherActor :type Actor%20Object%20Reference) (OtherComp :type Primitive%20Component%20Object%20Reference) (OtherBodyIndex :type Integer))
  ;[1 1 1] Can AJ Interact?
  (Utilities|Casting|CastToAJprefab_Blueprint OtherActor)
  (bind _asdwgame_mode (Utilities|Casting|CastToDWGameMode (Game|GetGameMode)))
  (if (Variables|/Game/UI/DWGameMode.DWGameMode_C|GetIsAJChar _asdwgame_mode)
    (bind _asdwgame_mode_2 (Utilities|Casting|CastToDWGameMode (Game|GetGameMode)))
    (Variables|/Game/UI/DWGameMode.DWGameMode_C|SetAJInteract _asdwgame_mode_2 false)
    (Widget|RemovefromParent (Variables|Default|GetClickPrompt))))

(event EventTick
  (params (DeltaSeconds :type Float%20%28single-precision%29))
  ;[1 1 1] Remove Prompt at Character Change
  (bind _asdwgame_mode (Utilities|Casting|CastToDWGameMode (Game|GetGameMode)))
  (if (not (Variables|/Game/UI/DWGameMode.DWGameMode_C|GetIsAJChar _asdwgame_mode))
    (Widget|RemovefromParent (Variables|Default|GetClickPrompt))))

(fn ConstructionScript)