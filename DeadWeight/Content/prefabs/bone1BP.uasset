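; Collectible bone pickup actor that records its collection in the game instance.
; On Collect component overlap, it destroys itself, passes NewBone to AddBones on DWGameInstance and sets that instance's Bone1 flag.
; BeginPlay destroys the actor if Bone1 is already set, so the picked-up bone does not reappear.
; The flag is hard-coded, tying this Blueprint to one specific bone.
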(event OnComponentBeginOverlap(Collect)
  (params (OverlappedComponent :type Primitive%20Component%20Object%20Reference) (OtherActor :type Actor%20Object%20Reference) (OtherComp :type Primitive%20Component%20Object%20Reference) (OtherBodyIndex :type Integer) (bFromSweep :type Boolean) (SweepResult :type Hit%20Result%20Structure%20%28by%20ref%29))
  ;[1 1 1] Bone Pick Up
  (Actor|DestroyActor)
  (bind _asdwgame_instance (Utilities|Casting|CastToDWGameInstance (Game|GetGameInstance)))
  (Default|AddBones _asdwgame_instance (Variables|Default|GetNew%20Bone))
  (Variables|/Game/UI/DWGameInstance.DWGameInstance_C|SetBone1 _asdwgame_instance true))

(event EventBeginPlay
  ;[1 1 1] No Bone - Already Picked Up
  (bind _asdwgame_instance (Utilities|Casting|CastToDWGameInstance (Game|GetGameInstance)))
  (if (Variables|/Game/UI/DWGameInstance.DWGameInstance_C|GetBone1 _asdwgame_instance)
    (Actor|DestroyActor)))

(fn ConstructionScript)